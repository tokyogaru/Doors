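; Game mode that owns the player's health, death and respawn, plus crate and key counters.
; It creates the health HUD on BeginPlay, and damage and heal events clamp Vida, with zero-point damage (Min) triggering MuerteJugador.
; An OnDestroyed binding respawns and possesses a new character after a delay, restores health and rebinds.
; Each key count creates another key HUD widget.
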(event Custom|OnDestroyed_
  (params (DestroyedActor :type Actor%20Object%20Reference))
  (bind _returnvalue (Game|GetPlayerController 0))
  (bind _asbp_player_controller_class (Utilities|Casting|CastToBP_PlayerControllerClass _returnvalue))
  (Utilities|FlowControl|Delay 1.0)
  (bind _returnvalue_2 (Game|SpawnActorfromClass "/Game/Blueprints/BP_Character.BP_Character_C" (Variables|Default|GetSpawn%20Transform) "Undefined" "MultiplyWithRoot" 0 0))
  (bind _output_get (Variables|/Game/Blueprints/BP_PlayerControllerClass.BP_PlayerControllerClass_C|SetAs%20BP%20Character _asbp_player_controller_class _returnvalue_2))
  (Pawn|Possess _asbp_player_controller_class _output_get)
  (Variables|Default|SetVida (Variables|Default|GetVidaMax))
  (CallFunction|SavePawnLocation))

(event EventBeginPlay
  (bind _returnvalue (UserInterface|CreateWidget "/Game/HUD/HUD_Vida.HUD_Vida_C" (Variables|Default|GetOwning%20Player)))
  (bind _output_get (Variables|Default|SetHUD%20Reference _returnvalue))
  (UserInterface|Viewport|AddtoViewport _output_get 0))

(event EventSavePawnLocation
  (bind _asbp_character (Utilities|Casting|CastToBP_Character (Game|GetPlayerCharacter 0)))
  (Game|BindEventtoOnDestroyed _asbp_character (delegate Custom|OnDestroyed_)))

(event EventSalud
  (Variables|Default|SetVida (Math|Float|Clamp(Float) (+ (Variables|Default|GetVida) (Variables|Default|GetCantidadRecuperacion)) (Variables|Default|GetMin) (Variables|Default|GetVidaMax))))

(event EventConteoLlaves
  (bind _returnvalue (UserInterface|CreateWidget "/Game/HUD/HUD_Llaves.HUD_Llaves_C"))
  (bind _output_get (Variables|Default|SetHUDKeys _returnvalue))
  (UserInterface|Viewport|AddtoViewport _output_get 0)
  (bind _result (Math|Integer|IncrementInt (Variables|Default|GetKeys))
    (:%20%20
      (bind _output_get_2 (Variables|Default|SetKeys _result))
      (Development|PrintString (Utilities|String|ToString(Integer) _output_get_2)))))

(event EventDaño
  (bind _min (Variables|Default|GetMin))
  (bind _output_get (Variables|Default|SetVida (Math|Float|Clamp(Float) (- (Variables|Default|GetVida) (Variables|Default|GetCantidadDaño)) _min (Variables|Default|GetVidaMax))))
  (if (<= _output_get _min)
    (Default|MuerteJugador (stale Custom|OnDestroyed_ _output_get))
    (CallFunction|SavePawnLocation)))

(event EventAgregarCajas
  (bind _result (Math|Integer|IncrementInt (Variables|Default|GetCajas))
    (:%20%20
      (Development|PrintString (Utilities|String|ToString(Integer) _result)))))

(fn ConstructionScript)