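; BP_Door is a lockable, interactable door that swings open and closed once its key has been collected.
; RecolectKey sets the key flag, which lets Interact toggle the target yaw between closed and open and play a door sound.
; Tick continuously interpolates the Scene component's yaw toward that target at SpeedDoor, while BeginPlay applies the configured material to the mesh.
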(event EventRecolectKey
  (Variables|Default|SetGetKey? true))

(event EventBeginPlay
  (Rendering|Material|SetMaterial (Variables|Default|GetStaticMesh) 0 (Variables|Default|GetMaterial)))

(event EventInteract
  (if (Variables|Default|GetGetKey?)
    (if (Variables|Default|GetIsOpened)
      (Variables|Default|SetTargetAngle 0.0)
      (Variables|Default|SetIsOpened false)
      (else
        (Variables|Default|SetTargetAngle 9e+01)
        (Variables|Default|SetIsOpened true)))
    (Audio|PlaySound2D "/Game/Assets/SFX/door_Cue.door_Cue" 1.0 1.0 0.0 0 0)))

(event EventTick
  (params (DeltaSeconds :type Float%20%28single-precision%29))
  (Transformation|SetRelativeRotation (Variables|Default|GetScene) (Math|Rotator|MakeRotator 0.0 0.0 (Math|Interpolation|FInterpTo (.yaw (Variables|/Script/Engine.SceneComponent|GetRelativeRotation (Variables|Default|GetScene))) (Variables|Default|GetTargetAngle) DeltaSeconds (Variables|Default|GetSpeedDoor))) false false))

(fn ConstructionScript)