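; BP_Button is a pressure button that sinks when triggered and has Spawn show a keys message.
; Tick interpolates Cube1's height toward TargetLocation, which the Box overlap events set.
; In IsCharacter mode, BP_Character overlap presses it if IsTouched is set, fires the message once, and exit raises it.
; In BP_Caja mode, only exit changes the target; the CajaTouched press logic is disconnected.
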(event OnComponentEndOverlap(Box)
  (params (OverlappedComponent :type Primitive%20Component%20Object%20Reference) (OtherActor :type Actor%20Object%20Reference) (OtherComp :type Primitive%20Component%20Object%20Reference) (OtherBodyIndex :type Integer))
  (if (Variables|Default|GetIsCharacter?)
    (Utilities|Casting|CastToBP_Character OtherActor)
    (Variables|Default|SetTargetLocation 5.0)
    (else
      (Utilities|Casting|CastToBP_Caja OtherActor)
      (Variables|Default|SetTargetLocation 5.0))))

(event OnComponentBeginOverlap(Box)
  (params (OverlappedComponent :type Primitive%20Component%20Object%20Reference) (OtherActor :type Actor%20Object%20Reference) (OtherComp :type Primitive%20Component%20Object%20Reference) (OtherBodyIndex :type Integer) (bFromSweep :type Boolean) (SweepResult :type Hit%20Result%20Structure%20%28by%20ref%29))
  (if (Variables|Default|GetIsCharacter?)
    (Utilities|Casting|CastToBP_Character OtherActor)
    (if (Variables|Default|GetIsTouched?)
      (Variables|Default|SetTargetLocation -6.0)
      (Utilities|FlowControl|DoOnce false
        (:Completed
          (Class|BPIButtons|SpawnKeys(Message) (Variables|Default|GetSpawn))))
      (else
        (Variables|Default|SetTargetLocation 5.0)))
    (else
      (Utilities|Casting|CastToBP_Caja OtherActor)
      (if true
        _))))

(event EventTick
  (params (DeltaSeconds :type Float%20%28single-precision%29))
  (Transformation|SetRelativeLocation (Variables|Default|GetCube1) (Math|Vector|MakeVector 0.0 0.0 (Math|Interpolation|FInterpTo (.z (Variables|/Script/Engine.SceneComponent|GetRelativeLocation (Variables|Default|GetCube1))) (Variables|Default|GetTargetLocation) DeltaSeconds (Variables|Default|GetButtonSpeed))) false false))

(fn ConstructionScript)