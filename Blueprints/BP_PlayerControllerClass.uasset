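; Player controller that routes Enhanced Input to the possessed BP_Character.
; On BeginPlay it casts and caches the controlled pawn, then adds the IMC_Character mapping context.
; Move, look (with inverted Y), jump and interact actions call the character's own movement, camera, jump and door functions, so the gameplay logic lives in the character.
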(event Input|EnhancedActionEvents|EnhancedInputActionIA_Move
  (params (ActionValue :type Vector%202D%20Structure) (ElapsedSeconds :type Float%20%28double-precision%29) (TriggeredSeconds :type Float%20%28double-precision%29) (InputAction :type Input%20Action%20Object%20Reference :default "/Game/Input/IA_Move.IA_Move"))
  (bind _as_bp_character (Variables|Default|GetAs%20BP%20Character))
  (:Triggered
    (Default|ArribaAbajo _as_bp_character (.y ActionValue))
    (Default|IzquierdaDerecha _as_bp_character (.x ActionValue))))

(event Input|EnhancedActionEvents|EnhancedInputActionIA_Look
  (params (ActionValue :type Vector%202D%20Structure) (ElapsedSeconds :type Float%20%28double-precision%29) (TriggeredSeconds :type Float%20%28double-precision%29) (InputAction :type Input%20Action%20Object%20Reference :default "/Game/Input/IA_Look.IA_Look"))
  (:Triggered
    (Default|Mirar (Variables|Default|GetAs%20BP%20Character) (.x ActionValue) (* -1.0 (.y ActionValue)))))

(event Input|EnhancedActionEvents|EnhancedInputActionIA_Jump
  (params (ActionValue :type Boolean) (ElapsedSeconds :type Float%20%28double-precision%29) (TriggeredSeconds :type Float%20%28double-precision%29) (InputAction :type Input%20Action%20Object%20Reference :default "/Game/Input/IA_Jump.IA_Jump"))
  (:Triggered
    (Default|EventJump (Variables|Default|GetAs%20BP%20Character) ActionValue)))

(event Input|EnhancedActionEvents|EnhancedInputActionIA_InteractionObjects
  (params (ActionValue :type Boolean) (ElapsedSeconds :type Float%20%28double-precision%29) (TriggeredSeconds :type Float%20%28double-precision%29) (InputAction :type Input%20Action%20Object%20Reference :default "/Game/Input/IA_InteractionObjects.IA_InteractionObjects"))
  (:Started
    (Default|EventDoor (Variables|Default|GetAs%20BP%20Character))))

(event EventBeginPlay
  (bind _returnvalue (Game|GetPlayerController 0))
  (bind _returnvalue_2 (PlayerController|LocalPlayerSubsystems|GetEnhancedInputLocalPlayerSubsystem _returnvalue))
  (bind _asbp_character (Utilities|Casting|CastToBP_Character (Pawn|GetControlledPawn)))
  (Variables|Default|SetAs%20BP%20Character _asbp_character)
  (Utilities|IsValid _returnvalue_2
    (:Is%20Valid
      (Input|AddMappingContext _returnvalue_2 "/Game/Input/InputMappingContext/IMC_Character.IMC_Character" 0 "(bIgnoreAllPressedKeysUntilRelease=True,bForceImmediately=False)"))))

(fn ConstructionScript)