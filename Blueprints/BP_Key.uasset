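; BP_Key is a collectible key actor that a player picks up by interacting with it.
; On begin play it applies its material to the cube and sets visibility and actor collision from variables, so a key can start hidden or non-solid.
; Interacting sends a collect message to its referenced Door and a key-count message to the game mode, then destroys the key.
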(event EventBeginPlay
  (Rendering|Material|SetMaterial (Variables|Default|GetCube) 0 (Variables|Default|GetMaterial))
  (Rendering|SetVisibility (Variables|Default|GetCube) (Variables|Default|GetNew%20Visibility) false)
  (Collision|SetActorEnableCollision (Variables|Default|GetNew%20Visibility_0)))

(event EventInteract
  (Class|BPIKeys|RecolectKey(Message) (Variables|Default|GetDoor))
  (Class|BPIKeys|ConteoLlaves(Message) (Game|GetGameMode))
  (Actor|DestroyActor))

(fn ConstructionScript)